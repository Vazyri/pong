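; BP_Paddle is a player-controlled paddle that moves its PaddleLeft component from Enhanced Input.
; On BeginPlay it adds the IMC_Paddle mapping context to the owning player controller's input subsystem.
; The IA_Paddle action scales its value by PaddleSpeed and applies it as a local offset, without sweep or delta-time scaling.
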(event Input|EnhancedActionEvents|EnhancedInputActionIA_Paddle
  (params (ActionValue :type Float%20%28double-precision%29) (ElapsedSeconds :type Float%20%28double-precision%29) (TriggeredSeconds :type Float%20%28double-precision%29) (InputAction :type Input%20Action%20Object%20Reference :default "/Game/input/IA_Paddle.IA_Paddle"))
  (Transformation|AddLocalOffset (Variables|Pawn|GetPaddle_Left) (Math|Conversions|ToVector(Float) (* ActionValue (Variables|Default|GetpaddleSpeed))) false false))

(event EventBeginPlay
  (bind _asplayer_controller (Utilities|Casting|CastToPlayerController (Pawn|GetController)))
  (Utilities|IsValid (PlayerController|LocalPlayerSubsystems|GetEnhancedInputLocalPlayerSubsystem _asplayer_controller)
    (:Is%20Valid
      (Input|AddMappingContext (PlayerController|LocalPlayerSubsystems|GetEnhancedInputLocalPlayerSubsystem _asplayer_controller) "/Game/input/IMC_Paddle.IMC_Paddle" 0 "(bIgnoreAllPressedKeysUntilRelease=True,bForceImmediately=False,bNotifyUserSettings=False)"))))

(event Collision|EventActorBeginOverlap
  (params (OtherActor :type Actor%20Object%20Reference)))

(event EventTick
  (params (DeltaSeconds :type Float%20%28single-precision%29)))

(fn ConstructionScript)